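; BP_PuzzleCube is a physics-driven puzzle cube whose motion state and collision can be read or set from outside.
; GetTrajectory returns the actor's transform and the Cube component's linear and angular velocities, with control rotation zeroed.
; SetTrajectory teleports the actor to a given location and rotation, then overwrites both velocities.
; SetCollisionResponse changes the Cube's response on a given collision channel.
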(event EventBeginPlay)

(event Collision|EventActorBeginOverlap
  (params (OtherActor :type Actor%20Object%20Reference)))

(event EventTick
  (params (DeltaSeconds :type Float%20%28single-precision%29)))

(event EventSetTrajectory
  (params (Location :type Vector%20%28by%20ref%29 :default "0, 0, 0") (Rotation :type Rotator%20%28by%20ref%29 :default "0, 0, 0") (ControlRotation :type Rotator%20%28by%20ref%29 :default "0, 0, 0") (LinearVelocity :type Vector%20%28by%20ref%29 :default "0, 0, 0") (AngularVelocity :type Vector%20%28by%20ref%29 :default "0, 0, 0"))
  (bind _cube (Variables|Default|GetCube))
  (Transformation|SetActorLocationAndRotation Location Rotation false true)
  (Class|PrimitiveComponent|SetAllPhysicsLinearVelocity _cube LinearVelocity false)
  (Class|PrimitiveComponent|SetAllPhysicsAngularVelocityinDegrees _cube AngularVelocity false))

(event EventSetCollisionResponse
  (params (Channel :type ECollisionChannel%20Enum :default "ECC_WorldStatic") (Response :type ECollisionResponse%20Enum :default "ECR_Ignore"))
  (Collision|SetCollisionResponsetoChannel (Variables|Default|GetCube) Channel Response))

(fn ConstructionScript)

(fn GetTrajectory
  (bind _cube (Variables|Default|GetCube))
  (bind _returnvalue (Physics|GetPhysicsLinearVelocity _cube "None"))
  (return (Transformation|GetActorLocation) (Transformation|GetActorRotation) "0, 0, 0" _returnvalue (Physics|GetPhysicsAngularVelocityinDegrees _cube "None")))
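; BP_ProximityDoor is a puzzle-element door that opens while the first-person character is inside its trigger and closes when they leave.
; On BeginPlay it stores the mesh's relative transform as the closed position.
; Trigger overlaps play or reverse a timeline that lerps the door mesh between the closed transform and a separate open transform.
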(event OnComponentBeginOverlap(Trigger)
  (params (OverlappedComponent :type Primitive%20Component%20Object%20Reference) (OtherActor :type Actor%20Object%20Reference) (OtherComp :type Primitive%20Component%20Object%20Reference) (OtherBodyIndex :type Integer) (bFromSweep :type Boolean) (SweepResult :type Hit%20Result%20Structure%20%28by%20ref%29))
  (Utilities|Casting|CastToBP_FirstPersonCharacter OtherActor)
  (bind _dooropen_ (Timeline|DoorAnimation Play)
    (:Update
      (Transformation|SetRelativeTransform (Variables|Default|GetDoorMesh) (Math|Transform|Lerp(Transform) (Variables|Default|GetDoorClosedPosition) (Variables|Default|GetDoorOpenPosition) _dooropen_) false false))))

(event OnComponentEndOverlap(Trigger)
  (params (OverlappedComponent :type Primitive%20Component%20Object%20Reference) (OtherActor :type Actor%20Object%20Reference) (OtherComp :type Primitive%20Component%20Object%20Reference) (OtherBodyIndex :type Integer))
  (Utilities|Casting|CastToBP_FirstPersonCharacter OtherActor)
  (bind _dooropen_ (Timeline|DoorAnimation Reverse)
    (:Update
      (Transformation|SetRelativeTransform (Variables|Default|GetDoorMesh) (Math|Transform|Lerp(Transform) (Variables|Default|GetDoorClosedPosition) (Variables|Default|GetDoorOpenPosition) _dooropen_) false false))))

(event EventBeginPlay
  (Variables|Default|SetDoorClosedPosition (Transformation|GetRelativeTransform (Variables|Default|GetDoorMesh))))

(fn ConstructionScript)
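; BP_Door is a puzzle element door that slides or swings between closed and open poses.
; It stores the mesh's starting relative transform as the closed position on BeginPlay.
; OpenDoor plays a timeline that lerps the mesh toward DoorOpenPosition, and CloseDoor reverses the same timeline to return it.
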(event Custom|Open%20Door
  (bind _dooropen_ (Timeline|DoorAnimation Play)
    (:Update
      (Transformation|SetRelativeTransform (Variables|Default|GetDoorMesh) (Math|Transform|Lerp(Transform) (Variables|Default|GetDoorClosedPosition) (Variables|Default|GetDoorOpenPosition) _dooropen_) false false))))

(event Custom|Close%20Door
  (bind _dooropen_ (Timeline|DoorAnimation Reverse)
    (:Update
      (Transformation|SetRelativeTransform (Variables|Default|GetDoorMesh) (Math|Transform|Lerp(Transform) (Variables|Default|GetDoorClosedPosition) (Variables|Default|GetDoorOpenPosition) _dooropen_) false false))))

(event EventBeginPlay
  (Variables|Default|SetDoorClosedPosition (Transformation|GetRelativeTransform (Variables|Default|GetDoorMesh))))

(fn ConstructionScript)